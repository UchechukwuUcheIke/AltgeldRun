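; GM_Gamemode is a game mode that builds a chain of BP_Tile actors, starting from a tile already placed in the level.
; On BeginPlay it finds that first tile, passes it a reference to itself and spawns four more.
; SpawnTiles places each new tile at the previous tile's SpawnPoint and hands it the game mode reference, so the chain can be extended from the latest end point.
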(event EventBeginPlay
  (bind _outactors (Actor|GetAllActorsOfClass "/Game/BP_Tile.BP_Tile_C"))
  (bind _output_get (Variables|Default|SetBaseTile_Ref (Utilities|Array|Get(acopy) _outactors)))
  (Variables|/Game/BP_Tile.BP_Tile_C|SetGame_Ref _output_get self)
  (Variables|Default|SetNextSpawnPoint (Transformation|GetWorldLocation (Variables|/Game/BP_Tile.BP_Tile_C|GetSpawn_Point _output_get)))
  (CallFunction|SpawnTiles 4))

(event EventTick
  (params (DeltaSeconds :type Float%20%28single-precision%29)))

(fn ConstructionScript)

(fn SpawnTiles
  (params (Amount :type Integer))
  (for _index (range 0 (- Amount 1))
    (bind _returnvalue (Game|SpawnActorfromClass "/Game/BP_Tile.BP_Tile_C" (Math|Transform|MakeTransform (Variables|Default|GetNextSpawnPoint) "0, 0, 0" "1.000000,1.000000,1.000000") "Undefined" "MultiplyWithRoot" 0 0))
    (Variables|/Game/BP_Tile.BP_Tile_C|SetGame_Ref _returnvalue self)
    (Variables|Default|SetNextSpawnPoint (Transformation|GetWorldLocation (Variables|/Game/BP_Tile.BP_Tile_C|GetSpawn_Point _returnvalue)))))