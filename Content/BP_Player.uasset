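; Player Blueprint that moves constantly along world X and switches between three lanes, in the style of a lane runner.
; BeginPlay adds the Enhanced Input mapping context, and the left and right move actions step a Slot index clamped to the three lanes.
; Each Tick, UpdatePosition eases the root's Y toward the selected lane with FInterpTo, then a world offset scaled by MoveSpeed and delta time advances X.
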(event Input|EnhancedActionEvents|EnhancedInputActionIA_MoveLeft
  (params (ActionValue :type Boolean) (ElapsedSeconds :type Float%20%28double-precision%29) (TriggeredSeconds :type Float%20%28double-precision%29) (InputAction :type Input%20Action%20Object%20Reference :default "/Game/IA_MoveLeft.IA_MoveLeft"))
  (if (not (<= (Variables|Default|GetSlot) 0))
    (bind _result (Math|Integer|DecrementInt (Variables|Default|GetSlot))
      (:%20%20
        (Variables|Default|SetSlot _result)))))

(event Input|EnhancedActionEvents|EnhancedInputActionIA_MoveRight
  (params (ActionValue :type Boolean) (ElapsedSeconds :type Float%20%28double-precision%29) (TriggeredSeconds :type Float%20%28double-precision%29) (InputAction :type Input%20Action%20Object%20Reference :default "/Game/IA_MoveRight.IA_MoveRight"))
  (if (not (>= (Variables|Default|GetSlot) 2))
    (bind _result (Math|Integer|IncrementInt (Variables|Default|GetSlot))
      (:%20%20
        (Variables|Default|SetSlot _result)))))

(event EventBeginPlay
  (bind _asplayer_controller (Utilities|Casting|CastToPlayerController (Pawn|GetController)))
  (Utilities|IsValid (PlayerController|LocalPlayerSubsystems|GetEnhancedInputLocalPlayerSubsystem _asplayer_controller)
    (:Is%20Valid
      (Input|AddMappingContext (PlayerController|LocalPlayerSubsystems|GetEnhancedInputLocalPlayerSubsystem _asplayer_controller) "/Game/IMC_InputMapping.IMC_InputMapping" 0 "(bIgnoreAllPressedKeysUntilRelease=True,bForceImmediately=False,bNotifyUserSettings=False)"))))

(event Collision|EventActorBeginOverlap
  (params (OtherActor :type Actor%20Object%20Reference)))

(event EventTick
  (params (DeltaSeconds :type Float%20%28single-precision%29))
  (CallFunction|UpdatePosition)
  (Transformation|AddActorWorldOffset (Math|Vector|MakeVector (* (Variables|Default|GetMoveSpeed) DeltaSeconds) 0.0 0.0)))

(fn ConstructionScript)

(fn UpdatePosition
  (bind _slot (Variables|Default|GetSlot))
  (bind _defaultsceneroot (Variables|Default|GetDefaultSceneRoot))
  (bind _defaultsceneroot_2 (Variables|Default|GetDefaultSceneRoot))
  (bind _returnvalue (Transformation|GetWorldLocation _defaultsceneroot))
  (bind _returnvalue_2 (Transformation|GetWorldLocation _defaultsceneroot_2))
  (bind _returnvalue_3 (Utilities|Select :Index _slot :Option%200 -2e+02 :Option%201 0.0 :Option%202 2e+02))
  (if (!= (.y _returnvalue_2) _returnvalue_3)
    (Transformation|SetWorldLocation _defaultsceneroot_2 (Math|Vector|MakeVector (.x _returnvalue) (Math|Interpolation|FInterpTo (.y _returnvalue_2) _returnvalue_3 (Utilities|Time|GetWorldDeltaSeconds) 8.0) (.z _returnvalue)) false false)))